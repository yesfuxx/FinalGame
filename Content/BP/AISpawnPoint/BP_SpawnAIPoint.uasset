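; Placeable AI spawn point that spawns a set number of monsters at its own location and rotation.
; On BeginPlay, the server starts a looping timer that spawns one monster per interval, passing attack interval, max HP and controller type, until the count runs out.
; The construction script picks the monster class from an array by monster type, with only Mutant mapped; its controller-type switch just reassigns Chase to itself.
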(event `self.ReceiveBeginPlay`
  (if (`KismetSystemLibrary.IsServer`)
    (bind _returnvalue (`KismetSystemLibrary.K2_SetTimerDelegate` (delegate `Spawn Monster`) (`self.Spawn Interval`) true))
    (set `self.Timer Handle` _returnvalue)))

(event `Spawn Monster`
  (if (<= (`self.Spawn Num`) 0)
    (`KismetSystemLibrary.K2_ClearAndInvalidateTimerHandle` (`self.Timer Handle`))
    (else
      (`|SpawnActorFromClass` (`self.Monster Class`) (`KismetMathLibrary.MakeTransform` (`self.K2_GetActorLocation`) (`self.K2_GetActorRotation`)) "Undefined" "OverrideRootScale" null (`self.Attack Interval`) (`self.Max HP`) (`self.Controller Type`) null)
      (`/Engine/EditorBlueprintResources/StandardMacros.DecrementInt` (`self.Spawn Num`)))))

(fn `UserConstructionScript`
  (`|ExecutionSequence`
    (:`then_0`
      (switch `/Game/BP/AISpawnPoint/E_MonsterType` (`self.Monster Type`)
        (:`NewEnumerator0`
          (set `self.Monster Class` (`|GetArrayItem` (`self.Monster Class Arr`))))))
    (:`then_1`
      (switch `/Game/BP/AI/E_AIControllerType` (`self.Controller Type`)
        (:`NewEnumerator0`
          (set `self.Controller Type` "NewEnumerator0"))))))