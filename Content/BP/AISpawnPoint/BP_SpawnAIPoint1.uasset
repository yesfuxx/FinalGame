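; BP_SpawnAIPoint1 is an AI spawn point that releases a set number of monsters at its own location and rotation.
; The SpawnAI event stores count, type, controller type, max HP and interval, picks the class from MonsterClassArr by type index, and starts a looping timer.
; Each tick of that timer spawns one monster with the HP and controller type, clearing itself once the count runs out.
; The construction script only handles the Mutant and Chase cases.
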(event `Spawn AI`
  (params (`Msg Spawn Num` :type Integer) (`Msg Monster Type` :type "/Game/BP/AISpawnPoint/E_MonsterType Enum" :default "NewEnumerator0") (`Msg AIController Type` :type "/Game/BP/AI/E_AIControllerType Enum" :default "NewEnumerator2") (`Msg Max HP` :type "Float (double-precision)") (`Msg Spawn Interval` :type "Float (double-precision)"))
  (set `self.Spawn Num` `Msg Spawn Num`)
  (bind _output_get (set `self.Monster Type` `Msg Monster Type`))
  (set `self.AIController Type` `Msg AIController Type`)
  (set `self.Max HP` `Msg Max HP`)
  (set `self.Spawn Interval` `Msg Spawn Interval`)
  (set `self.Monster Class` (`|GetArrayItem` (`self.Monster Class Arr`) (`KismetMathLibrary.Conv_ByteToInt` _output_get)))
  (bind _returnvalue (`KismetSystemLibrary.K2_SetTimerDelegate` (delegate `Spawn Monster`) (`self.Spawn Interval`) true))
  (set `self.Timer Handle` _returnvalue))

(event `Spawn Monster`
  (if (> (`self.Spawn Num`) 0)
    (`|SpawnActorFromClass` :`Class` (`self.Monster Class`) :`SpawnTransform` (`KismetMathLibrary.MakeTransform` (`self.K2_GetActorLocation`) (`self.K2_GetActorRotation`)) :`CollisionHandlingOverride` "Undefined" :`TransformScaleMethod` "OverrideRootScale" :`Max HP` (`self.Max HP`) :`Controller Type` (`self.AIController Type`) :`Instigator` null)
    (`/Engine/EditorBlueprintResources/StandardMacros.DecrementInt` (`self.Spawn Num`))
    (else
      (`KismetSystemLibrary.K2_ClearAndInvalidateTimerHandle` (`self.Timer Handle`)))))

(fn `UserConstructionScript`
  (`|ExecutionSequence`
    (:`then_0`
      (switch `/Game/BP/AISpawnPoint/E_MonsterType` (`self.Monster Type`)
        (:`NewEnumerator0`
          (set `self.Monster Class` (`|GetArrayItem` (`self.Monster Class Arr`))))))
    (:`then_1`
      (switch `/Game/BP/AI/E_AIControllerType` (`self.AIController Type`)
        (:`NewEnumerator0`
          (set `self.AIController Type` "NewEnumerator0"))))))