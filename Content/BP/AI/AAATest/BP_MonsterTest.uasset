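; BP_MonsterTest is a test AI monster that chases the first BP_LittleGirl in the level and plays an attack animation up close.
; Chase starts shortly after BeginPlay, using SimpleMoveToActor through the AI controller.
; Box overlap with the girl sets IsAttack and replays the montage, delayed by its length, until she leaves, then Chase resumes.
; No damage is applied: Attack is empty, and the StopMovementImmediately call is disconnected.
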(event `self.ReceiveBeginPlay`
  (`KismetSystemLibrary.Delay` 0.2)
  (`self.Chase`))

(event `Chase`
  (bind _outactors (`GameplayStatics.GetAllActorsOfClass` "/Game/BP/Character/BP_LittleGirl.BP_LittleGirl_C"))
  (`AIBlueprintHelperLibrary.SimpleMoveToActor` (`AIBlueprintHelperLibrary.GetAIController` self) (`|GetArrayItem` _outactors)))

(event `Attack`)

(event `self.Box.OnComponentBeginOverlap`
  (params (OverlappedComponent :type "PrimitiveComponent Object Reference") (OtherActor :type "Actor Object Reference") (OtherComp :type "PrimitiveComponent Object Reference") (OtherBodyIndex :type Integer) (bFromSweep :type Boolean) (SweepResult :type "HitResult Structure (by ref)"))
  (cast `/Game/BP/Character/BP_LittleGirl` OtherActor)
  (set `self.Is Attack?` true)
  (bind _returnvalue (`self.PlayAnimMontage` "/Game/BP/AI/AAATest/NewAnimMontage.NewAnimMontage" :!label _label))
  (`KismetSystemLibrary.Delay` _returnvalue)
  (if (`self.Is Attack?`)
    (goto _label)
    (else
      (`self.Chase`))))

(event `self.Box.OnComponentEndOverlap`
  (params (OverlappedComponent :type "PrimitiveComponent Object Reference") (OtherActor :type "Actor Object Reference") (OtherComp :type "PrimitiveComponent Object Reference") (OtherBodyIndex :type Integer))
  (cast `/Game/BP/Character/BP_LittleGirl` OtherActor)
  (set `self.Is Attack?` false))

(fn `UserConstructionScript`)