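; Base monster AI character that attacks players, takes damage and awards score to BP_LittleGirl killers, with its AI controller class picked by ControllerType at construction.
; On server Tick, a timer starts a random attack while AttackSign is set; per-type delays open a hit window in which a matching overlap deals damage once.
; Damage reduces HP and spawns floating numbers locally or via a client event; death disables Pawn and WorldDynamic collision, mirrored through OnRep_Die.
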(event `Set Has Attacked`
  (params (`Has Attacked` :type Boolean))
  (set `self.Has Attacked` `Has Attacked`))

(event `Server Set Has Attacked`
  (params (`Has Attacked` :type Boolean))
  (`KismetSystemLibrary.PrintString` "Server Set Has Attacked")
  (`self.Set Has Attacked` `Has Attacked`))

(event `Server Set Attack Sign`
  (params (Attack :type Boolean))
  (`self.Set Attack Sign` Attack))

(event `self.ReceiveBeginPlay`)

(event `Set Attack Sign`
  (params (Attack :type Boolean))
  (set `self.Attack Sign` Attack))

(event `self.ReceiveTick`
  (params (DeltaSeconds :type "Float (single-precision)"))
  (if (`KismetSystemLibrary.IsServer`)
    (`KismetSystemLibrary.PrintString` (`KismetStringLibrary.Conv_BoolToString` (`self.Has Attacked`)) true true (struct :`R` 0.073421 :`G` 1.0 :`A` 1.0) 0.0)
    (set `self.Attack Timer` (+ DeltaSeconds (`self.Attack Timer`)))
    (if (>= (`self.Attack Timer`) (`self.Attack Interval`))
      (if (`self.Attack Sign`)
        (`self.Attack To Do`)
        (set `self.Attack Timer` 0.0)))))

(event `Attack To Do`
  (`|ExecutionSequence`
    (:`then_0`
      ;[1 1 1] Random Attack Type
      (bind _output_get (set `self.Attack Index` (`KismetMathLibrary.RandomIntegerInRange` 0 (- (`self.Attack Type Num`) 1))))
      (set `self.Do Attack` true)
      (`KismetSystemLibrary.K2_SetTimerDelegate` (delegate `Stop Attack To Do`) (`|GetArrayItem` (`self.Attack Type Anin Time`) _output_get))
      (set `self.Has Attacked` true))
    (:`then_1`
      (`KismetSystemLibrary.Delay` (`|GetArrayItem` (`self.Attack Type Anin Time Can Attack`) (`self.Attack Index`)))
      (set `self.Has Attacked` false))))

(event `Stop Attack To Do`
  (set `self.Do Attack` false)
  (set `self.Has Attacked` true))

(event `Overlap To Do`
  (params (Player :type "/Game/BP/Character/BP_LittleGirl Object Reference") (`Attack Index` :type Integer))
  ;[1 1 1] 怪物拳头接触
  (if (== `Attack Index` (`self.Attack Index`))
    (if (`self.Do Attack`)
      (if (not (`self.Has Attacked`))
        (set `self.Has Attacked` true)
        (`self.Damage Monster Attack` Player)))))

(event `Damage Monster Attack`
  (params (`Damaged Actor` :type "/Game/BP/Character/BP_LittleGirl Object Reference"))
  ;[1 1 1] Attack Damage
  (`/Engine/EditorBlueprintResources/StandardMacros.IsValid` `Damaged Actor`
    (:`Is Valid`
      (`GameplayStatics.ApplyDamage` `Damaged Actor` (`|GetArrayItem` (`self.Attack Type Damage`) (`self.Attack Index`))))))

(event `self.ReceiveAnyDamage`
  (params (Damage :type "Float (single-precision)") (DamageType :type "DamageType Object Reference") (InstigatedBy :type "Controller Object Reference") (DamageCauser :type "Actor Object Reference"))
  (bind _returnvalue (- (`self.Current HP`) Damage))
  ;[1 1 1] Is Dead?
  (if (<= _returnvalue 0.0)
    (`/Engine/EditorBlueprintResources/StandardMacros.DoOnce` false
      (:`Completed`
        (`self.CreateDamageNumber` InstigatedBy Damage)
        (`self.After Dead To Do`)
        ;[1 1 1] Add Score After Dead
        (bind _asbp_little_girl (cast `/Game/BP/Character/BP_LittleGirl` (`Controller.K2_GetPawn` InstigatedBy)))
        (`/Game/BP/Character/BP_LittleGirl.Add Score` _asbp_little_girl (`self.Score`))))
    (else
      (set `self.Current HP` _returnvalue)
      (`self.CreateDamageNumber` InstigatedBy Damage))))

(event `After Dead To Do`
  (bind _capsulecomponent (`self.CapsuleComponent`))
  (set `self.Die` true)
  (`PrimitiveComponent.SetCollisionResponseToChannel` _capsulecomponent "ECC_WorldDynamic" "ECR_Ignore")
  (`PrimitiveComponent.SetCollisionResponseToChannel` _capsulecomponent "ECC_Pawn" "ECR_Ignore"))

(event `CreateDamageNumber`
  (params (Controller :type "Controller Object Reference") (Damage :type "Float (double-precision)"))
  ;[1 1 1] Create Float Damage Number
  (if (`Controller.IsLocalController` Controller)
    (`self.Create Float Damage Number` Damage)
    (else
      (`self.Client Create Float Damage Number` Damage))))

(event `Client Create Float Damage Number`
  (params (Damage :type "Float (double-precision)"))
  ;[1 1 1] Create Float Damage Number
  (if (not (`KismetSystemLibrary.IsServer`))
    (`self.Create Float Damage Number` Damage)))

(event `Create Float Damage Number`
  (params (Damage :type "Float (double-precision)"))
  ;[1 1 1] Create Float Damage Number
  (bind _aswbp_help_float (cast `/Game/BP/UI/Game/FloatDamageNumber/WBP_HelpFloat` (`WidgetComponent.GetUserWidgetObject` (`self.WidgetFloatDamageParent`))))
  (`/Game/BP/UI/Game/FloatDamageNumber/WBP_HelpFloat.Create Float Damage Number` _aswbp_help_float Damage))

(fn `Get Current Take Damage`
  (returns (Damage :type "Float (double-precision)"))
  (return (`|GetArrayItem` (`self.Attack Type Damage`) (`self.Attack Index`))))

(fn `OnRep_Die`
  (`self.After Dead To Do`))

(fn `Update Speed`
  (params (`New Speed` :type "Float (double-precision)"))
  (set `CharacterMovementComponent.MaxWalkSpeed` `New Speed` (`self.CharacterMovement`)))

(fn `UserConstructionScript`
  (bind _controllers (`self.Controllers`))
  (`|ExecutionSequence`
    (:`then_0`
      (set `self.Current HP` (`self.Max HP`))
      (switch `/Game/BP/AI/E_ControllerType` (`self.Controller Type`)
        (:`NewEnumerator2`
          (set `self.AIControllerClass` null))
        (:`NewEnumerator0`
          (set `self.AIControllerClass` (`|GetArrayItem` _controllers)))
        (:`NewEnumerator1`
          (set `self.AIControllerClass` (`|GetArrayItem` _controllers 1)))))))