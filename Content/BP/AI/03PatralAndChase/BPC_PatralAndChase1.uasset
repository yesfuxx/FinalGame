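; AI controller for a patrol-and-chase enemy that runs the BT_PatralAndChase behavior tree on possess.
; AI Perception target updates maintain a list of sensed Player-tagged actors, writing the first one added to an empty list into the TargetActor blackboard key.
; Losing a player starts a delayed timer, cancelled by any new target update, that clears the key if the list is empty.
; Other perception, noise and hearing handlers only print debug strings or read stimuli.
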(event `self.ReceivePossess`
  (params (PossessedPawn :type "Pawn Object Reference"))
  (`self.RunBehaviorTree` "/Game/BP/AI/03PatralAndChase/BT_PatralAndChase.BT_PatralAndChase"))

(event `self.ReceiveTick`
  (params (DeltaSeconds :type "Float (single-precision)"))
  (`parent.ReceiveTick` DeltaSeconds))

(event `self.AIPerception.OnTargetPerceptionUpdated`
  (params (Actor :type "Actor Object Reference") (Stimulus :type "AIStimulus Structure"))
  (bind _tags (`Actor.Tags` Actor))
  (bind _actors (`self.Actors`))
  (`KismetSystemLibrary.K2_ClearAndInvalidateTimerHandle` (`self.Handle`))
  (if (`KismetArrayLibrary.Array_IsValidIndex` _tags)
    (if (== (`|GetArrayItem` _tags) "Player")
      (if (`.bSuccessfullySensed` (break `AIStimulus` Stimulus))
        (if (not (`KismetArrayLibrary.Array_Contains` (`self.Actors`) Actor))
          (`KismetArrayLibrary.Array_Add` _actors Actor)
          (if (== (`KismetArrayLibrary.Array_Length` (`self.Actors`)) 1)
            (`BlackboardComponent.SetValueAsObject` (`self.Blackboard`) "TargetActor" (`|GetArrayItem` (`self.Actors`)))))
        (else
          (`KismetArrayLibrary.Array_RemoveItem` _actors Actor)
          (bind _returnvalue (`KismetSystemLibrary.K2_SetTimerDelegate` (delegate `CustomEvent_0`) 5.0))
          (set `self.Handle` _returnvalue))))))

(event `CustomEvent_0`
  (if (== (`KismetArrayLibrary.Array_Length` (`self.Actors`)) 0)
    (`BlackboardComponent.SetValueAsObject` (`self.Blackboard`) "TargetActor" null)))

(event `self.AIPerception.OnPerceptionUpdated`
  (params (UpdatedActors :type "Array of Actor Object Reference (by ref)"))
  (`KismetSystemLibrary.PrintString` "Hello")
  (for _array_element UpdatedActors
    (bind _info (`AIPerceptionComponent.GetActorsPerception` (`self.AIPerception`) _array_element))
    (for _array_element_2 (`.LastSensedStimuli` (break `ActorPerceptionBlueprintInfo` _info))
      (set `self.NewVar_0` (`.bSuccessfullySensed` (break `AIStimulus` _array_element_2)))
      (`KismetSystemLibrary.PrintString` "11111111"))))

(event `self.PawnNoiseEmitter.OnComponentActivated`
  (params (Component :type "ActorComponent Object Reference") (bReset :type Boolean))
  (`KismetSystemLibrary.PrintString` "444444444"))

(event `self.PawnSensing.OnHearNoise`
  (params (Instigator :type "Pawn Object Reference") (Location :type "Vector Structure (by ref)") (Volume :type "Float (single-precision)"))
  (`KismetSystemLibrary.PrintString` "3333333"))

(fn `UserConstructionScript`
  (`parent.UserConstructionScript`))