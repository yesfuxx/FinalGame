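; BPC_Chase is an AI controller that runs the BT_Chase behavior tree when it possesses a pawn.
; BeginPlay and the FIndTargetActor event are empty.
; Disconnected logic would pick the nearest "Player"-tagged actor by squared distance, with debug prints, and write it to the TargetActor blackboard key.
; As wired, that search never runs, so this controller does not set the chase target.
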(event `self.ReceivePossess`
  (params (PossessedPawn :type "Pawn Object Reference"))
  (`self.RunBehaviorTree` "/Game/BP/AI/AIChase/BT_Chase.BT_Chase"))

(event `self.ReceiveBeginPlay`)

(event `FInd Target Actor`)

(fn `UserConstructionScript`)