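; Boss fire-strike actor that, as wired, only stamps an impact crater on the ground where it spawns.
; BeginPlay traces along its up axis for the surface type, which selects a DT_Material row with a default fallback.
; SpawnDecals then attaches a fading decal to the hit component with randomized frame, size and roll.
; The telegraph-then-explosion sequence, with particle toggling, sound, camera shake and radial damage, is disconnected and never runs.
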(event `Spawn Decals`
  (params (Location :type "Vector Structure") (AttachToComponent :type "SceneComponent Object Reference"))
  (bind (_surface _impactparticlefx _impactsound _impactdecal _decalsize) (break `/Game/BP/Effect/S_MaterialData` (`self.Material Values`)))
  (bind (_surface_2 _impactparticlefx_2 _impactsound_2 _impactdecal_2) (break `/Game/BP/Effect/S_MaterialData` (`self.Material Values`)))
  ;[1 1 1] 弹坑
  (`/Engine/EditorBlueprintResources/StandardMacros.IsValid` _impactdecal_2
    (:`Is Valid`
      (bind _returnvalue (`KismetMaterialLibrary.CreateDynamicMaterialInstance` _impactdecal_2))
      (bind _output_get (set `self.Impact Decal Mat` _returnvalue))
      (`/Engine/EditorBlueprintResources/StandardMacros.IsValid` _output_get
        (:`Is Valid`
          (`MaterialInstanceDynamic.SetScalarParameterValue` _output_get "Frame" (`KismetMathLibrary.Conv_IntToDouble` (`KismetMathLibrary.RandomIntegerInRange` 2 4)))
          (bind _returnvalue_2 (`GameplayStatics.SpawnDecalAttached` (`self.Impact Decal Mat`) (* (select `/Game/BP/Effect/E_ProjectileSIze` (cast `/Game/BP/Effect/E_ProjectileSIze` (`KismetMathLibrary.Conv_IntToByte` (`KismetMathLibrary.RandomIntegerInRange` 0 2))) :`NewEnumerator0` (2.0 2.0 2.0) :`NewEnumerator1` (4.0 4.0 4.0) :`NewEnumerator2` (6.0 6.0 6.0) :!type "Vector Structure") (* (`KismetMathLibrary.MakeVector` (.x _decalsize) (.y _decalsize) (.z _decalsize)) (`KismetMathLibrary.RandomFloatInRange` 0.75 1.9))) AttachToComponent "None" Location (`KismetMathLibrary.MakeRotator` (`KismetMathLibrary.RandomFloatInRange` 0.0 360.0) (.pitch (`KismetMathLibrary.Conv_VectorToRotator` (* (`SceneComponent.GetUpVector` (`self.Scene`)) -1))) (.yaw (`KismetMathLibrary.Conv_VectorToRotator` (* (`SceneComponent.GetUpVector` (`self.Scene`)) -1)))) "KeepWorldPosition" (`KismetMathLibrary.RandomFloatInRange` 3.0 8.0)))
          (`/Engine/EditorBlueprintResources/StandardMacros.IsValid` _returnvalue_2
            (:`Is Valid`
              (`DecalComponent.SetFadeOut` _returnvalue_2 (`KismetMathLibrary.RandomFloatInRange` 3.0 8.0) 5.0 false))))))))

(event `Set FX Type`
  (bind _returnvalue (`|GetDataTableRow` "/Game/BP/Effect/DT_Material.DT_Material" (`|GetEnumeratorName` (`self.SurfaceType Feedback`)))
    (:`then`
      (set `self.Material Values` _returnvalue))
    (:`RowNotFound`
      (bind _returnvalue_2 (`|GetDataTableRow` "/Game/BP/Effect/DT_Material.DT_Material" "SurfaceType_Default")
        (:`then`
          _)
        (:`RowNotFound`
          _))
      (set `self.Material Values` _returnvalue_2))))

(event `self.ReceiveBeginPlay`
  (bind _returnvalue (`self.K2_GetActorLocation`))
  (bind _returnvalue_2 (`SceneComponent.GetUpVector` (`self.Scene`)))
  (bind (_outhit _returnvalue_3) (`KismetSystemLibrary.LineTraceSingleForObjects` :`Start` (+ _returnvalue (* _returnvalue_2 10.0)) :`End` (+ (* _returnvalue_2 -10.0) _returnvalue) :`ObjectTypes` (`|MakeArray` "ObjectTypeQuery1" :!type "EObjectTypeQuery Enum") :`DrawDebugType` "ForDuration"))
  (bind (_bblockinghit _binitialoverlap _time _distance _location _impactpoint _normal _impactnormal _physmat _hitactor _hitcomponent) (`GameplayStatics.BreakHitResult` _outhit))
  (set `self.SurfaceType Feedback` (select `bool` _returnvalue_3 :`false` "SurfaceType_Default" :`true` (`PhysicalMaterial.SurfaceType` _physmat)))
  (`self.Set FX Type`)
  (`self.Spawn Decals` _impactpoint _hitcomponent))

(fn `Set Active`
  (params (`Boom Active` :type Boolean) (`Pre Active` :type Boolean))
  (`ActorComponent.SetActive` (`self.Explosion_GrenadeLauncher_Boss`) `Boom Active` false)
  (`ActorComponent.SetActive` (`self.P_FakeLight_Ground_mobile`) `Pre Active` false)
  (`ActorComponent.SetActive` (`self.P_FakeLight_Ground_mobile1`) `Pre Active` false)
  (`ActorComponent.SetActive` (`self.P_FakeLight_Ground_mobile2`) `Pre Active` false)
  (`ActorComponent.SetActive` (`self.P_Circle_ChargeUp_Fire_Phase2`) `Pre Active` false))

(fn `UserConstructionScript`)