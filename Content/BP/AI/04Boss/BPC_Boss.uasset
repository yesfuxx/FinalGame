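; AI controller for the boss that runs the BT_Boss behavior tree on possess and starts the blackboard attack Type at its initial value.
; ChangeBossAttackType toggles Type between two attack modes and updates the controlled BP_BaseAICharacter's AttackTypeIndex and Attack flag to match.
; Tick prints the current attack type and target actor on screen as debug output.
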(event `self.ReceiveBeginPlay`
  (bind _asbp_base_aicharacter (cast `/Game/BP/AI/Monster/BP_BaseAICharacter` (`self.K2_GetPawn`)))
  (set `self.AIPawn` _asbp_base_aicharacter))

(event `self.ReceiveTick`
  (params (DeltaSeconds :type "Float (single-precision)"))
  (`KismetSystemLibrary.PrintString` (`|GetEnumeratorNameAsString` (cast `/Game/BP/AI/04Boss/E_BossAttackType` (`BlackboardComponent.GetValueAsEnum` (`self.Blackboard`) "Type"))) true true (struct :`R` 1.0 :`G` 0.876578 :`A` 1.0) 0.0)
  (`KismetSystemLibrary.PrintString` (`KismetSystemLibrary.GetDisplayName` (`BlackboardComponent.GetValueAsObject` (`self.Blackboard`) "TargetActor")) true true (struct :`R` 1.0 :`G` 0.122561 :`B` 0.146437 :`A` 1.0) 0.0))

(event `self.ReceivePossess`
  (params (PossessedPawn :type "Pawn Object Reference"))
  (`self.RunBehaviorTree` "/Game/BP/AI/04Boss/BT_Boss.BT_Boss")
  (`BlackboardComponent.SetValueAsEnum` (`self.Blackboard`) "Type" 1))

(fn `Change Boss Attack Type`
  (bind _blackboard (`self.Blackboard`))
  (bind _aipawn (`self.AIPawn`))
  (bind _returnvalue (`BlackboardComponent.GetValueAsEnum` (`self.Blackboard`) "Type"))
  (if (== _returnvalue 1)
    (`BlackboardComponent.SetValueAsEnum` _blackboard "Type" 2)
    (set `/Game/BP/AI/Monster/BP_BaseAICharacter.Attack Type Index` 3 _aipawn)
    (set `/Game/BP/AI/Monster/BP_BaseAICharacter.Attack` true _aipawn)
    (else
      (if (== _returnvalue 2)
        _
        (else
          _))
      (`BlackboardComponent.SetValueAsEnum` _blackboard "Type" 1)
      (set `/Game/BP/AI/Monster/BP_BaseAICharacter.Attack Type Index` 0 _aipawn)
      (set `/Game/BP/AI/Monster/BP_BaseAICharacter.Attack` false _aipawn))))

(fn `UserConstructionScript`)