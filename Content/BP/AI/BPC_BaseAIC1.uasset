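; Base AI controller that runs a patrol-and-chase behavior tree on possess and feeds it player sightings from AI Perception.
; Sensing an actor tagged Player cancels the lose-sight timer and sets the HasLineOfSight and TargetActor blackboard keys.
; Any other perception update, including one for a non-player actor, starts a timer that clears both keys after the LineOfSightTimer delay.
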(event `self.ReceivePossess`
  (params (PossessedPawn :type "Pawn Object Reference"))
  (`self.RunBehaviorTree` "/Game/BP/AI/03PatralAndChase/BT_PatralAndChase.BT_PatralAndChase"))

(event `self.ReceiveBeginPlay`)

(event `self.AIPerception.OnTargetPerceptionUpdated`
  (params (Actor :type "Actor Object Reference") (Stimulus :type "AIStimulus Structure"))
  (bind _blackboard (`self.Blackboard`))
  (`KismetSystemLibrary.PrintString` "Hello")
  (if (and (`self.ActorHasTag` Actor "Player") (`.bSuccessfullySensed` (break `AIStimulus` Stimulus)))
    (`KismetSystemLibrary.K2_ClearAndInvalidateTimerHandle` (`self.Timer`))
    (`BlackboardComponent.SetValueAsBool` _blackboard (`self.HasLineOfSight`) true)
    (`BlackboardComponent.SetValueAsObject` _blackboard (`self.TargetActor`) Actor)
    (else
      (bind _returnvalue (`KismetSystemLibrary.K2_SetTimerDelegate` (delegate `StartEnemyTimer`) (`self.Line Of Sight Timer`)))
      (set `self.Timer` _returnvalue))))

(event `self.AIPerception.OnPerceptionUpdated`
  (params (UpdatedActors :type "Array of Actor Object Reference (by ref)")))

(event `StartEnemyTimer`
  (bind _blackboard (`self.Blackboard`))
  (`BlackboardComponent.SetValueAsBool` _blackboard (`self.HasLineOfSight`) false)
  (`BlackboardComponent.SetValueAsObject` _blackboard (`self.TargetActor`) null))

(fn `UserConstructionScript`)