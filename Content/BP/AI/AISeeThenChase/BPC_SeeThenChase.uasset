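; AI controller that runs the BT_SeeThenChase behavior tree on possess, apparently for an enemy that spots and chases the player.
; Successfully sensing a Player-tagged actor clears the timer and writes HasLineOfSight and TargetActor to the Blackboard.
; A timer event would clear both keys, but the code that starts it is unconnected, so the target is never released here.
; Perception events also print debug strings.
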(event `self.ReceivePossess`
  (params (PossessedPawn :type "Pawn Object Reference"))
  (`self.RunBehaviorTree` "/Game/BP/AI/AISeeThenChase/BT_SeeThenChase.BT_SeeThenChase"))

(event `self.ReceiveBeginPlay`)

(event `self.AIPerception.OnTargetPerceptionUpdated`
  (params (Actor :type "Actor Object Reference") (Stimulus :type "AIStimulus Structure"))
  (bind _blackboard (`self.Blackboard`))
  (`KismetSystemLibrary.PrintString` "Hello")
  (if (and (`self.ActorHasTag` Actor "Player") (`.bSuccessfullySensed` (break `AIStimulus` Stimulus)))
    (`KismetSystemLibrary.K2_ClearAndInvalidateTimerHandle` (`self.Timer`))
    (`BlackboardComponent.SetValueAsBool` _blackboard (`self.HasLineOfSight`) true)
    (`BlackboardComponent.SetValueAsObject` _blackboard (`self.TargetActor`) Actor)))

(event `self.AIPerception.OnPerceptionUpdated`
  (params (UpdatedActors :type "Array of Actor Object Reference (by ref)"))
  (`KismetSystemLibrary.PrintString` (`KismetStringLibrary.Conv_IntToString` (`KismetArrayLibrary.Array_Length` UpdatedActors)) true true (struct :`R` 1.0 :`B` 0.035027 :`A` 1.0) 2222222336.0))

(event `StartEnemyTimer`
  (bind _blackboard (`self.Blackboard`))
  (`BlackboardComponent.SetValueAsBool` _blackboard (`self.HasLineOfSight`) false)
  (`BlackboardComponent.SetValueAsObject` _blackboard (`self.TargetActor`) null))

(fn `UserConstructionScript`)