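; AI controller that runs the BT_HasPerceptionChase behavior tree on possess for perception-driven chasing.
; Perception updates keep an Actors list of sensed BP_LittleGirl characters, adding or removing them only while they are not dead.
; SetTheNearestActor picks the closest actor from a given array by distance and writes it to the TargetActor blackboard key, but nothing in this graph calls it.
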(event `self.ReceivePossess`
  (params (PossessedPawn :type "Pawn Object Reference"))
  (`self.RunBehaviorTree` "/Game/BP/AI/02HasPerceptionChase/BT_HasPerceptionChase.BT_HasPerceptionChase"))

(event `self.AIPerception.OnTargetPerceptionUpdated`
  (params (Actor :type "Actor Object Reference") (Stimulus :type "AIStimulus Structure"))
  (bind _actors (`self.Actors`))
  (bind _asbp_little_girl (cast `/Game/BP/Character/BP_LittleGirl` Actor))
  (if (not (`/Game/BP/Character/BP_LittleGirl.Death` _asbp_little_girl))
    (if (`.bSuccessfullySensed` (break `AIStimulus` Stimulus))
      (if (not (`KismetArrayLibrary.Array_Contains` _actors Actor))
        (`KismetArrayLibrary.Array_Add` _actors Actor))
      (else
        (`KismetArrayLibrary.Array_RemoveItem` _actors Actor)))))

(fn `Set The Nearest Actor`
  (params (Actors :type "Array of Actor Object Reference"))
  (locals (`Temp Length` :type "Float (double-precision)") (`Temp Actor` :type "Actor Object Reference"))
  (for (_array_element _array_index) Actors
    (if (== _array_index 0)
      (bind _returnvalue (`KismetMathLibrary.VSize` (- (`self.K2_GetActorLocation` _array_element) (`self.K2_GetActorLocation`))))
      (set `local.Temp Length` _returnvalue)
      (set `local.Temp Actor` _array_element)
      (`KismetSystemLibrary.PrintString` "111111111")
      (elif (< _returnvalue (`local.Temp Length`))
        (set `local.Temp Length` _returnvalue)
        (set `local.Temp Actor` _array_element)
        (`KismetSystemLibrary.PrintString` "22222222222222222"))))
  (`BlackboardComponent.SetValueAsObject` (`self.Blackboard`) "TargetActor" (`local.Temp Actor`)))

(fn `UserConstructionScript`)