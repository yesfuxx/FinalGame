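; Anim notify that deals melee damage from monster attack animations, evaluated only on the server.
; It runs a debug-drawn vertical box trace in front of the mesh, compensating for 90-degree mesh yaw and using tunable offsets and box size, mostly scaled by mesh scale.
; A hit on the queried object type receives damage from the owning BP_BaseAICharacter's GetCurrentTakeDamage.
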(fn `Received_Notify`
  (params (MeshComp :type "SkeletalMeshComponent Object Reference") (Animation :type "AnimSequenceBase Object Reference"))
  (returns (ReturnValue :type Boolean))
  (locals (Scale :type "Float (double-precision)" :default 0.0))
  (bind _returnvalue (`SceneComponent.K2_GetComponentRotation` MeshComp))
  (bind _scale (`local.Scale`))
  (bind _z (.z (+ (`SceneComponent.K2_GetComponentLocation` MeshComp) (* (`KismetMathLibrary.GetForwardVector` (`KismetMathLibrary.MakeRotator` (.roll _returnvalue) (.pitch _returnvalue) (+ (.yaw _returnvalue) 90.0))) (* 90.0 (`local.Scale`))))))
  (bind _returnvalue_2 (+ (`self.Offset X`) (.x (+ (`SceneComponent.K2_GetComponentLocation` MeshComp) (* (`KismetMathLibrary.GetForwardVector` (`KismetMathLibrary.MakeRotator` (.roll _returnvalue) (.pitch _returnvalue) (+ (.yaw _returnvalue) 90.0))) (* 90.0 (`local.Scale`)))))))
  (bind _returnvalue_3 (+ (`self.Offset Y`) (.y (+ (`SceneComponent.K2_GetComponentLocation` MeshComp) (* (`KismetMathLibrary.GetForwardVector` (`KismetMathLibrary.MakeRotator` (.roll _returnvalue) (.pitch _returnvalue) (+ (.yaw _returnvalue) 90.0))) (* 90.0 (`local.Scale`)))))))
  (if (`KismetSystemLibrary.IsServer`)
    (set `local.Scale` (.x (`SceneComponent.K2_GetComponentScale` MeshComp)))
    (bind (_outhit _returnvalue_4) (`KismetSystemLibrary.BoxTraceSingleForObjects` :`Start` (`KismetMathLibrary.MakeVector` _returnvalue_2 _returnvalue_3 (+ _z (* (`self.Up`) _scale))) :`End` (`KismetMathLibrary.MakeVector` _returnvalue_2 _returnvalue_3 (+ _z (* _scale (`self.Down`)))) :`HalfSize` (* (`self.Box Scale`) (`local.Scale`)) :`Orientation` _returnvalue :`ObjectTypes` (`|MakeArray` "ObjectTypeQuery12" :!type "EObjectTypeQuery Enum") :`DrawDebugType` "ForDuration" :`TraceColor` (struct :`R` 1.0 :`G` 0.099843 :`A` 1.0) :`DrawTime` 1.0))
    (if _returnvalue_4
      (bind _asbp_base_aicharacter (cast `/Game/BP/AI/Monster/BP_BaseAICharacter` (`ActorComponent.GetOwner` MeshComp)))
      (`GameplayStatics.ApplyDamage` (`.HitActor` (`GameplayStatics.BreakHitResult` _outhit)) (`/Game/BP/AI/Monster/BP_BaseAICharacter.Get Current Take Damage` _asbp_base_aicharacter))
      (return false)
      (else
        (return false)))))