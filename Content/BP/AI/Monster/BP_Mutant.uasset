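; BP_Mutant is an AI monster that attacks with its hands, building on attack logic inherited from its parent class.
; The construction script attaches left and right collision components to the mesh's hand sockets.
; On the server only, hand overlaps call OverlapToDo with the other actor and an attack index identifying the hand.
; Tick and AttacktoDo defer to the parent, and leftover disconnected debug and damage nodes never run.
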(event `self.ReceiveTick`
  (params (DeltaSeconds :type "Float (single-precision)"))
  (`parent.ReceiveTick` DeltaSeconds))

(event `self.Attack To Do`
  (`parent.Attack To Do`))

(event `self.CollisionRightHand.OnComponentBeginOverlap`
  (params (OverlappedComponent :type "PrimitiveComponent Object Reference") (OtherActor :type "Actor Object Reference") (OtherComp :type "PrimitiveComponent Object Reference") (OtherBodyIndex :type Integer) (bFromSweep :type Boolean) (SweepResult :type "HitResult Structure (by ref)"))
  (if (`KismetSystemLibrary.IsServer`)
    (`self.Overlap To Do` OtherActor)))

(event `self.CollisionRightHand.OnComponentEndOverlap`
  (params (OverlappedComponent :type "PrimitiveComponent Object Reference") (OtherActor :type "Actor Object Reference") (OtherComp :type "PrimitiveComponent Object Reference") (OtherBodyIndex :type Integer)))

(event `self.CollisionLeftHand.OnComponentBeginOverlap`
  (params (OverlappedComponent :type "PrimitiveComponent Object Reference") (OtherActor :type "Actor Object Reference") (OtherComp :type "PrimitiveComponent Object Reference") (OtherBodyIndex :type Integer) (bFromSweep :type Boolean) (SweepResult :type "HitResult Structure (by ref)"))
  (if (`KismetSystemLibrary.IsServer`)
    (`self.Overlap To Do` OtherActor 1)))

(event `self.CollisionLeftHand.OnComponentEndOverlap`
  (params (OverlappedComponent :type "PrimitiveComponent Object Reference") (OtherActor :type "Actor Object Reference") (OtherComp :type "PrimitiveComponent Object Reference") (OtherBodyIndex :type Integer)))

(fn `UserConstructionScript`
  (`parent.UserConstructionScript`)
  (`SceneComponent.K2_AttachToComponent` (`self.CollisionRightHand`) (`self.Mesh`) "RightHandSocket" "KeepRelative" "KeepRelative" "KeepRelative" true)
  (`SceneComponent.K2_AttachToComponent` (`self.CollisionLeftHand`) (`self.Mesh`) "LeftHandSocket" "KeepRelative" "KeepRelative" "KeepRelative" true))