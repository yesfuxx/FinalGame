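; Maw boss monster that attacks by spawning BP_BossFire hazards on the ground around its AI target.
; Server-side Tick runs a flag-and-delay attack cycle while alive, randomly favoring a single fire over a scattered volley.
; SpawnFire reads TargetActor from the BPC_Boss blackboard and traces down to the floor beneath it.
; It spawns one randomly scaled fire there, or several at nearby reachable points with staggered spawn delays.
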(event `self.ReceiveBeginPlay`
  (`parent.ReceiveBeginPlay`)
  (bind _asbpc_boss (cast `/Game/BP/AI/04Boss/BPC_Boss` (`self.GetController`)))
  (set `self.BPC Boss Ref` _asbpc_boss))

(event `self.ReceiveTick`
  (params (DeltaSeconds :type "Float (single-precision)"))
  (`|ExecutionSequence`
    (:`then_0`
      (`parent.ReceiveTick` DeltaSeconds)
      (if (`self.Death`)
        _
        (elif (`KismetSystemLibrary.IsServer`)
          (`|ExecutionSequence`
            (:`then_0`
              (if (`self.Bool Sgin Boss`)
                (if (`self.Can Attack Boss`)
                  (set `self.Attack Type Index Boss` (`KismetMathLibrary.SelectInt` 0 1 (<= (`KismetMathLibrary.RandomFloatInRangeFromStream` 0.0 1000.0 (`KismetMathLibrary.MakeRandomStream` (`KismetMathLibrary.FTrunc` (`KismetSystemLibrary.GetGameTimeInSeconds`)))) 650.0)))
                  (set `self.Bool Sgin Boss` false)
                  (set `self.Attack Boss` true)
                  (`self.Spawn Fire`)
                  (`KismetSystemLibrary.Delay` (`|GetArrayItem` (`self.Attack Anim Time Boss`) (`self.Attack Type Index Boss`)))
                  (set `self.Attack Boss` false)
                  (`KismetSystemLibrary.Delay` (`|GetArrayItem` (`self.Attack Interval Boss`) (`self.Attack Type Index Boss`)))
                  (set `self.Bool Sgin Boss` true))))))))))

(event `self.After Death To Do`
  (`parent.After Death To Do`)
  (set `self.Attack Boss` false)
  (set `self.Bool Sgin Boss` false))

(event `Spawn Fire`
  (bind _returnvalue (`self.K2_GetActorLocation` (`self.Temp Target Actor`)))
  (bind _returnvalue_2 (`self.K2_GetActorLocation` (`self.Temp Target Actor`)))
  (bind _returnvalue_3 (select `int` (`KismetMathLibrary.RandomIntegerInRange` 0 5) :`0` (0.7 0.7 0.7) :`1` (0.8 1.0 0.8) :`2` (0.9 0.9 0.9) :`3` (1.0 1.0 1.0) :`4` (0.6 0.6 0.6) :`5` (0.4 0.4 0.4) :!type "Vector Structure"))
  (bind _x (.x _returnvalue_3))
  (bind _asactor (cast `Actor` (`BlackboardComponent.GetValueAsObject` (`AIController.Blackboard` (`self.BPC Boss Ref`)) "TargetActor")))
  (set `self.Temp Target Actor` _asactor)
  (if (== (`self.Attack Type Index Boss`) 0)
    (bind (_outhit _returnvalue_4) (`KismetSystemLibrary.LineTraceSingleForObjects` _returnvalue_2 (+ _returnvalue_2 (* (`KismetMathLibrary.GetForwardVector` (`KismetMathLibrary.MakeRotator` 0.0 -90.0)) 500.0)) (`|MakeArray` "ObjectTypeQuery1" :!type "EObjectTypeQuery Enum")))
    (if _returnvalue_4
      (`|SpawnActorFromClass` "/Game/BP/AI/04Boss/BP_BossFIre.BP_BossFire_C" (`KismetMathLibrary.MakeTransform` (select `bool` _returnvalue_4 :`false` _returnvalue_2 :`true` (`.ImpactPoint` (`GameplayStatics.BreakHitResult` _outhit))) (`KismetMathLibrary.MakeRotator` 0.0 0.0 (`KismetMathLibrary.RandomFloatInRange` 0.0 360.0)) _returnvalue_3) "Undefined" "OverrideRootScale" null 0.0 _x 400.0 75.0 self))
    (else
      (bind (_outhit_2 _returnvalue_5) (`KismetSystemLibrary.LineTraceSingleForObjects` _returnvalue (+ _returnvalue (* (`KismetMathLibrary.GetForwardVector` (`KismetMathLibrary.MakeRotator` 0.0 -90.0)) 500.0)) (`|MakeArray` "ObjectTypeQuery1" :!type "EObjectTypeQuery Enum")))
      (if _returnvalue_5
        (for _ (range (+ (`KismetMathLibrary.RandomIntegerInRange` 2 4) 1))
          (`|SpawnActorFromClass` "/Game/BP/AI/04Boss/BP_BossFIre.BP_BossFire_C" (`KismetMathLibrary.MakeTransform` (select `bool` _returnvalue_5 :`false` _returnvalue :`true` (`NavigationSystemV1.K2_GetRandomReachablePointInRadius` (`.ImpactPoint` (`GameplayStatics.BreakHitResult` _outhit_2)) 600.0 null null)) (`KismetMathLibrary.MakeRotator` 0.0 0.0 (`KismetMathLibrary.RandomFloatInRange` 0.0 360.0)) _returnvalue_3) "Undefined" "OverrideRootScale" null (`KismetMathLibrary.RandomFloatInRange` 0.5 3.0) _x 400.0 75.0 self))))))

(fn `UserConstructionScript`
  (`parent.UserConstructionScript`))