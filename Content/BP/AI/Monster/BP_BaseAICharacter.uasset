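; Base AI monster character that attacks in range and awards score to the BP_LittleGirl player who kills it.
; Construction sets scale, health and AI controller class from ControllerType.
; Server-side Tick cycles randomly chosen, timed attacks while AttackCheckBox has overlaps, counted on begin and end.
; AnyDamage drives health, damage numbers, hit markers and controller retargeting; death picks an animation, changes collision, destroys after a delay and triggers the GameMode's all-dead check.
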(event `self.ReceiveTick`
  (params (DeltaSeconds :type "Float (single-precision)"))
  (if (`self.Death`)
    _
    (elif (`KismetSystemLibrary.IsServer`)
      (`|ExecutionSequence`
        (:`then_0`
          (if (`self.Bool Sgin`)
            (if (`self.Can Attack`)
              (set `self.Attack Type Index` (`KismetMathLibrary.RandomIntegerInRangeFromStream` 0 (- (`KismetArrayLibrary.Array_Length` (`self.Attack Anim Time`)) 1) (`KismetMathLibrary.MakeRandomStream` (`KismetMathLibrary.FTrunc` (`KismetSystemLibrary.GetGameTimeInSeconds`)))))
              (set `self.Bool Sgin` false)
              (set `self.Attack` true)
              (`KismetSystemLibrary.Delay` (`|GetArrayItem` (`self.Attack Anim Time`) (`self.Attack Type Index`)))
              (set `self.Attack` false)
              (`KismetSystemLibrary.Delay` (`|GetArrayItem` (`self.Attack Interval`) (`self.Attack Type Index`)))
              (set `self.Bool Sgin` true))))))))

(event `self.Attack Check Box.OnComponentBeginOverlap`
  (params (OverlappedComponent :type "PrimitiveComponent Object Reference") (OtherActor :type "Actor Object Reference") (OtherComp :type "PrimitiveComponent Object Reference") (OtherBodyIndex :type Integer) (bFromSweep :type Boolean) (SweepResult :type "HitResult Structure (by ref)"))
  ;[1 1 1] Attack Check Box
  (`|ExecutionSequence`
    (:`then_1`
      (set `self.Can Attack` true)
      (`/Engine/EditorBlueprintResources/StandardMacros.IncrementInt` (`self.Help Check Set Attack`)))))

(event `self.Attack Check Box.OnComponentEndOverlap`
  (params (OverlappedComponent :type "PrimitiveComponent Object Reference") (OtherActor :type "Actor Object Reference") (OtherComp :type "PrimitiveComponent Object Reference") (OtherBodyIndex :type Integer))
  (bind _help_check_set_attack (`self.Help Check Set Attack`))
  ;[1 1 1] Attack Check Box
  (`/Engine/EditorBlueprintResources/StandardMacros.DecrementInt` _help_check_set_attack
    (:`  `
      (if (<= _help_check_set_attack 0)
        (set `self.Can Attack` false)))))

(event `self.ReceiveAnyDamage`
  (params (Damage :type "Float (single-precision)") (DamageType :type "DamageType Object Reference") (InstigatedBy :type "Controller Object Reference") (DamageCauser :type "Actor Object Reference"))
  (bind _returnvalue (`Controller.K2_GetPawn` InstigatedBy))
  (bind _returnvalue_2 (- (`self.Current HP`) Damage))
  (`/Engine/EditorBlueprintResources/StandardMacros.IsValid` InstigatedBy
    (:`Is Valid`
      (bind _asbp_little_girl (cast `/Game/BP/Character/BP_LittleGirl` (`Controller.K2_GetPawn` InstigatedBy)))
      (set `self.Damage From` _asbp_little_girl)
      (`|ExecutionSequence`
        (:`then_0`
          ;[1 1 1] HP Check
          (if (<= _returnvalue_2 0.0)
            (`/Engine/EditorBlueprintResources/StandardMacros.DoOnce` false
              (:`Completed`
                (set `self.Attack` false)
                ;[1 1 1] Add Player Score
                (`/Game/BP/Character/BP_LittleGirl.Add Score` (`self.Damage From`) (`self.Monster Score`))
                (`self.After Death To Do`)
                (`self.Is All AI Dead`)))
            (else
              (set `self.Current HP` _returnvalue_2))))
        (:`then_1`
          ;[1 1 1] Help Create Float Damage Text
          (if (not (`self.Death`))
            (`/Game/BP/Character/BP_LittleGirl.Help Create Damage Flote Text When Player Hit Monter` (`self.Damage From`) Damage self)))
        (:`then_2`
          ;[1 1 1] Comment
          (`/Engine/EditorBlueprintResources/StandardMacros.IsValid` InstigatedBy
            (:`Is Valid`
              (bind _asbpc_base_aicontroller (cast `/Game/BP/AI/Monster/BPC_BaseAIController` (`self.GetController`)))
              (`/Engine/EditorBlueprintResources/StandardMacros.IsValid` _returnvalue
                (:`Is Valid`
                  (bind _actors (`/Game/BP/AI/Monster/BPC_BaseAIController.Actors` _asbpc_base_aicontroller))
                  (if (not (`KismetArrayLibrary.Array_Contains` _actors _returnvalue))
                    (`KismetArrayLibrary.Array_Add` _actors _returnvalue)
                    (`/Game/BP/AI/Monster/BPC_BaseAIController.Refresh Nearest Target` _asbpc_base_aicontroller)))))))
        (:`then_3`
          ;[1 1 1] Show Hit Marker
          (`/Game/BP/Character/BP_LittleGirl.Owning Client Show Hit Marker` (`self.Damage From`)))))))

(event `After Death To Do`
  ;[1 1 1] Monster Death To DO
  (`self.Set Death Anim Index`)
  (set `self.Attack` false)
  (set `self.Death` true)
  (`PrimitiveComponent.SetCollisionProfileName` (`self.CapsuleComponent`) "AIDeath")
  (`KismetSystemLibrary.Delay` 5.0)
  (`self.K2_DestroyActor`))

(event `Is All AI Dead`
  (bind _asbp_game_mode (cast `/Game/BP/03Level/BP_GameMode` (`GameplayStatics.GetGameMode`)))
  (`/Game/BP/03Level/BP_GameMode.All AI Dead Check` _asbp_game_mode))

(event `Create Float Damage Text`
  (params (Damage :type "Float (double-precision)"))
  ;[1 1 1] Help Create Float Damage Text
  ;;[1 1 1] Create Float Damage Text UI
  (bind _aswbp_help_float (cast `/Game/BP/UI/Game/FloatDamageNumber/WBP_HelpFloat` (`WidgetComponent.GetUserWidgetObject` (`self.WidgetFloatDamageParent`))))
  (`/Game/BP/UI/Game/FloatDamageNumber/WBP_HelpFloat.Create Float Damage Number` _aswbp_help_float Damage))

(event `Set Death Anim Index`
  ;[1 1 1] Set Death Index
  (set `self.Death Ainm Index` (`KismetMathLibrary.RandomIntegerInRangeFromStream` 0 (- (`self.Death Anim Num`) 1) (`KismetMathLibrary.MakeRandomStream` (`KismetMathLibrary.FTrunc` (`KismetSystemLibrary.GetGameTimeInSeconds`))))))

(fn `Get Current Take Damage`
  (returns (Damage :type "Float (double-precision)"))
  (return (`|GetArrayItem` (`self.Attack Type Damage`) (`self.Attack Type Index`))))

(fn `OnRep_Die`
  (`self.After Death To Do`))

(fn `OnRep_In Attack Box`)

(fn `Update Speed`
  (params (`New Speed` :type "Float (double-precision)"))
  (set `CharacterMovementComponent.MaxWalkSpeed` `New Speed` (`self.CharacterMovement`)))

(fn `UserConstructionScript`
  (bind _controllers (`self.Controllers`))
  (bind _scale (`self.Scale`))
  (`self.SetActorScale3D` self (`KismetMathLibrary.MakeVector` _scale _scale _scale))
  (`|ExecutionSequence`
    (:`then_0`
      (set `self.Current HP` (`self.Max HP`))
      (switch `/Game/BP/AI/E_AIControllerType` (`self.Controller Type`)
        (:`NewEnumerator2`
          (set `self.AIControllerClass` "/Script/AIModule.AIController"))
        (:`NewEnumerator0`
          (set `self.AIControllerClass` (`|GetArrayItem` _controllers)))
        (:`NewEnumerator3`
          (set `self.AIControllerClass` (`|GetArrayItem` _controllers 1)))
        (:`NewEnumerator1`
          (set `self.AIControllerClass` (`|GetArrayItem` _controllers 2)))
        (:`NewEnumerator4`
          (set `self.AIControllerClass` (`|GetArrayItem` _controllers 3)))))))