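; Base AI controller for monsters that picks the nearest actor as the target and writes it to the Blackboard.
; RefreshNearestTarget passes the Actors list to SetNearestTarget, which linearly compares distances from the controller's own location and sets the TargetActor key.
; The IsValid check before that write is disconnected.
; Tick prints the current target's name to screen for debugging.
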(event `self.ReceiveTick`
  (params (DeltaSeconds :type "Float (single-precision)"))
  (`KismetSystemLibrary.PrintString` (`KismetSystemLibrary.GetDisplayName` (`BlackboardComponent.GetValueAsObject` (`self.Blackboard`) "TargetActor")) true true (struct :`R` 1.0 :`G` 0.188235 :`B` 0.308078 :`A` 1.0) 0.0))

(event `Refresh Nearest Target`
  (`self.Set Nearest Target` (`self.Actors`)))

(fn `Set Nearest Target`
  (params (Actors :type "Array of Actor Object Reference"))
  (locals (`Temp Length` :type "Float (double-precision)") (`Temp Actor` :type "Actor Object Reference"))
  (for (_array_element _array_index) Actors
    (if (== _array_index 0)
      (bind _returnvalue (`KismetMathLibrary.VSize` (- (`self.K2_GetActorLocation` _array_element) (`self.K2_GetActorLocation`))))
      (set `local.Temp Length` _returnvalue)
      (set `local.Temp Actor` _array_element)
      (elif (< _returnvalue (`local.Temp Length`))
        (set `local.Temp Length` _returnvalue)
        (set `local.Temp Actor` _array_element))))
  (`BlackboardComponent.SetValueAsObject` (`self.Blackboard`) "TargetActor" (`local.Temp Actor`)))

(fn `UserConstructionScript`)