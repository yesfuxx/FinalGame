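; BP_PlayerState holds a player's score, health and death flag, plus a copy of the player message list from BP_GameMode.
; AddScore accumulates score, while AddHP and CutHP clamp health between zero and MaxHP, with CutHP setting Dead at zero.
; A looping timer started on BeginPlay refreshes PlayerMsgList several times a second by polling GetPlayersMsg on the game mode.
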(event `self.ReceiveBeginPlay`
  (`self.Set Player MsgList`)
  (`KismetSystemLibrary.K2_SetTimerDelegate` (delegate `CustomEvent_0`) 0.2 true))

(event `self.ReceiveTick`
  (params (DeltaSeconds :type "Float (single-precision)")))

(event `CustomEvent_0`
  (`self.Set Player MsgList`))

(event `Set Player MsgList`
  (bind _asbp_game_mode (cast `/Game/BP/BP_GameMode` (`GameplayStatics.GetGameMode`)))
  (bind _playermsg (`/Game/BP/BP_GameMode.GetPlayersMsg` _asbp_game_mode))
  (set `self.PlayerMsgList` _playermsg))

(fn `Add HP`
  (params (`Add HP Value` :type Integer))
  (bind _max_hp (`self.Max HP`))
  (bind _returnvalue (+ `Add HP Value` (`self.Current HP`)))
  (if (> _returnvalue _max_hp)
    (set `self.Current HP` _max_hp)
    (else
      (set `self.Current HP` _returnvalue))))

(fn `Add Score`
  (params (`A Score` :type Integer))
  (set `self.Player Score` (+ `A Score` (`self.Player Score`))))

(fn `Cut HP`
  (params (`Cut HP Value` :type Integer))
  (bind _returnvalue (- (`self.Current HP`) `Cut HP Value`))
  (if (<= _returnvalue 0)
    (set `self.Current HP` 0)
    (set `self.Dead` true)
    (else
      (set `self.Current HP` _returnvalue))))

(fn `UserConstructionScript`)