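; BP_BaseDrug is a base Blueprint for drug items that provides a Cure event for child classes to override.
; On BeginPlay it calls the parent, then runs Cure on the network authority only, so the effect starts as soon as the actor begins play.
; The base Cure is a placeholder that only prints a debug message saying it should be overridden.
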(event `self.ReceiveBeginPlay`
  (`parent.ReceiveBeginPlay`)
  (`/Engine/EditorBlueprintResources/ActorMacros.Switch Has Authority`
    (:`Authority`
      (`self.Cure`))))

(event `Cure`
  (`KismetSystemLibrary.PrintString` "override cure" true true (struct :`R` 0.006373 :`G` 1.0 :`B` 0.026086 :`A` 1.0)))

(fn `UserConstructionScript`
  (`parent.UserConstructionScript`))