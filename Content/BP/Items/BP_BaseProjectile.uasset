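; BP_BaseProjectile is a base projectile Blueprint that sets up launch speed and randomized damage.
; Its construction script copies InitialSpeed into the ProjectileMovement component, then varies BaseDamage by a random fraction within plus or minus DamageOffset and rounds it.
; The IsServer check is disconnected, so this setup is not limited to the server, and the event graph holds only disabled stubs.
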(fn `Set Speed`
  (set `ProjectileMovementComponent.InitialSpeed` (`self.Initial Speed`) (`self.ProjectileMovement`)))

(fn `UserConstructionScript`
  (bind _damage_offset (`self.Damage Offset`))
  (`parent.UserConstructionScript`)
  (`self.Set Speed`)
  (set `self.Base Damage` (`KismetMathLibrary.Conv_IntToDouble` (`KismetMathLibrary.Round` (+ (* (`self.Base Damage`) (`KismetMathLibrary.RandomFloatInRange` (* _damage_offset -1.0) _damage_offset)) (`self.Base Damage`))))))