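; BP_Bandage is a healing item that restores HP to the player who instigated it.
; Its Cure event casts the instigator's PlayerState to BP_PlayerState, adds the truncated AddHPCount as HP, then restarts two particle effects through SpawnFX.
; Tick continuously interpolates the PLevelExitFire1 effect's scale toward zero, whether or not Cure has fired.
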(event `self.Cure`
  (bind _asbp_player_state (cast `/Game/BP/03Level/BP_PlayerState` (`Pawn.PlayerState` (`self.Instigator`))))
  (`/Game/BP/03Level/BP_PlayerState.Add HP` _asbp_player_state (`KismetMathLibrary.FTrunc` (`self.Add HP Count`)))
  (`self.Spawn FX`))

(event `Spawn FX`
  (`ActorComponent.SetActive` (`self.P_DeadMans_Loot`) true true)
  (`ActorComponent.SetActive` (`self.P_LevelExit_Fire1`) true true))

(event `self.ReceiveTick`
  (params (DeltaSeconds :type "Float (single-precision)"))
  (bind _p_levelexit_fire1 (`self.P_LevelExit_Fire1`))
  (`SceneComponent.SetRelativeScale3D` _p_levelexit_fire1 (`KismetMathLibrary.VInterpTo` (`SceneComponent.RelativeScale3D` _p_levelexit_fire1) (0.0 0.0 0.0) DeltaSeconds 0.5)))

(fn `UserConstructionScript`
  (`parent.UserConstructionScript`))