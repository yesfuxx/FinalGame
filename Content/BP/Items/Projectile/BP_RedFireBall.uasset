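; BP_RedFireBall is a fireball projectile that grows in flight, so longer flights give bigger, wider, more damaging explosions.
; A timeline started on BeginPlay drives actor scale.
; The first bounce stops it and uses that scale to size the explosion particles, radial damage and radius, alongside camera shake and sounds.
; It also draws a debug damage sphere, applies a fixed server-only impulse to the hit component, then hides and destroys itself after a delay.
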(event OnProjectileBounce(ProjectileMovement)
  (params (ImpactResult :type Hit%20Result%20Structure%20%28by%20ref%29) (ImpactVelocity :type Vector%20%28by%20ref%29 :default "0, 0, 0"))
  (bind (_bblockinghit _binitialoverlap _time _distance _location _impactpoint _normal _impactnormal _physmat _hitactor _hitcomponent) (Collision|BreakHitResult ImpactResult))
  (bind _returnvalue (* _normal -1))
  (bind _returnvalue_2 (Math|Conversions|RotationFromXVector _returnvalue))
  (bind (_roll _pitch _yaw) (Math|Rotator|BreakRotator _returnvalue_2))
  (Utilities|FlowControl|DoOnce false
    (:Completed
      (Utilities|FlowControl|Sequence
        (:then_0
          ;[1 1 1] 飞行时间越长 子弹越大 爆炸范围越大 伤害越高
          (bind _newtrack_0 (Timeline|Timeline_0 Stop)
            (:Update
              (Transformation|SetActorScale3D self (Math|Vector|MakeVector _newtrack_0 _newtrack_0 _newtrack_0)))))
        (:then_1
          (Camera|PlayWorldCameraShake "/Game/BP/Items/ExplosionShake.ExplosionShake_C" _location 0.0 1.5e+03)
          (bind _output_get (Variables|Default|SetScale_0 _newtrack_0))
          (Variables|Default|SetImpact%20Point _impactpoint)
          (Effects|SpawnEmitteratLocation "/Game/Asset/BallisticsVFX/Particles/Explosive/Explosion_FireBallSmoke.Explosion_FireBallSmoke" (Variables|Default|GetImpact%20Point) (Math|Rotator|MakeRotator (Math|Random|RandomFloatinRange 0.0 3.6e+02) _pitch _yaw) (Math|Vector|MakeVector (/ _output_get 5.0) (/ _output_get 5.0) (/ _output_get 5.0)) true "AutoRelease")
          (Audio|SpawnSoundatLocation "/Game/Asset/BallisticsVFX/SFX/Explodes/Explosions.Explosions" (Variables|Default|GetImpact%20Point) "0, 0, 0" 0.75 1.0 0.0 0 0)
          (Audio|SpawnSoundatLocation "/Game/BP/Sound/Projectile/GunGrenate.GunGrenate" (Variables|Default|GetImpact%20Point) "0, 0, 0" 0.75 1.0 0.0 0 0)
          (Utilities|FlowControl|Sequence
            (:then_0
              (Rendering|Debug|DrawDebugSphere (Variables|Default|GetImpact%20Point) (|(200+({29DC8815-44B2-C520-3AFD-05ADB63DFCF8}*70))) 12 "(R=1.000000,G=0.000000,B=0.000000,A=1.000000)" 1e+01)
              (Game|Damage|ApplyRadialDamage (|(BaseDamage+({29DC8815-44B2-C520-3AFD-05ADB63DFCF8}*5)) (Variables|Default|GetBase%20Damage)) (Variables|Default|GetImpact%20Point) (|(200+({29DC8815-44B2-C520-3AFD-05ADB63DFCF8}*70))) 0 0 self (Pawn|GetController (Variables|Default|GetInstigator)) false "ECC_Camera")
              (if (Networking|IsServer)
                (Physics|AddRadialImpulse _hitcomponent (Variables|Default|GetImpact%20Point) 5e+02 1e+06 "RIF_Linear" false)))
            (:then_1
              (Rendering|SetActorHiddenInGame self true)
              (Utilities|FlowControl|Delay 1.5)
              (Actor|DestroyActor))))))))

(event EventBeginPlay
  (|CallParentFunction)
  ;[1 1 1] 飞行时间越长 子弹越大 爆炸范围越大 伤害越高
  (bind _newtrack_0 (Timeline|Timeline_0 Play)
    (:Update
      (Transformation|SetActorScale3D self (Math|Vector|MakeVector _newtrack_0 _newtrack_0 _newtrack_0)))))

(event Collision|EventActorBeginOverlap
  (params (OtherActor :type Actor%20Object%20Reference))
  (|CallParentFunction OtherActor) ; This node is disabled and will not be called.\nDrag off pins to build functionality.
)

(event EventTick
  (params (DeltaSeconds :type Float%20%28single-precision%29))
  (|CallParentFunction DeltaSeconds) ; This node is disabled and will not be called.\nDrag off pins to build functionality.
)

(fn ConstructionScript
  (|CallParentFunction))