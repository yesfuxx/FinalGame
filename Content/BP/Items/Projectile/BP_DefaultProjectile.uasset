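; BP_DefaultProjectile is a projectile that damages BP_BaseAICharacter targets, doubling damage on "Head" bone hits.
; Tick activates the tracer flare once speed is low enough, then scales the mesh by velocity.
; Hit events push physics bodies using clamped velocity-based impulses.
; On projectile stop it switches collision to overlap, spawns BP_ImpactEffect, applies damage, and hides itself before delayed destruction; the impulse applied there is zero.
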(event `self.ReceiveHit`
  (params (MyComp :type "PrimitiveComponent Object Reference") (Other :type "Actor Object Reference") (OtherComp :type "PrimitiveComponent Object Reference") (bSelfMoved :type Boolean) (HitLocation :type "Vector Structure") (HitNormal :type "Vector Structure") (NormalImpulse :type "Vector Structure") (Hit :type "HitResult Structure (by ref)"))
  ;[1 1 1] 物理碰撞效果
  (if (`SceneComponent.IsSimulatingPhysics` OtherComp "None")
    (`PrimitiveComponent.AddImpulseAtLocation` OtherComp (`KismetMathLibrary.ClampVectorSize` (* (`self.GetVelocity`) 100.0) 0.0 100000.0) (`self.K2_GetActorLocation`) "None")))

(event `self.ReceiveTick`
  (params (DeltaSeconds :type "Float (single-precision)"))
  (bind _returnvalue (`KismetMathLibrary.VSize` (`MovementComponent.Velocity` (`self.ProjectileMovement`))))
  (bind _returnvalue_2 (`KismetMathLibrary.NormalizeToRange` _returnvalue 0.0 30000.0))
  ;[1 1 1] Tracer Scale per velocity + Tracer Flare
  (if (< _returnvalue_2 -1.0)
    _
    (elif (`ActorComponent.IsActive` (`self.TracerFlare`))
      (`SceneComponent.SetRelativeScale3D` (`self.Mesh`) (`KismetMathLibrary.Conv_DoubleToVector` (`KismetMathLibrary.MapRangeClamped` _returnvalue 0.0 10000.0 0.1 2.0)))
      (elif (<= _returnvalue_2 0.2)
        (`ActorComponent.Activate` (`self.TracerFlare`) false)))))

(event `self.ProjectileMovement.OnProjectileStop`
  (params (ImpactResult :type "HitResult Structure (by ref)"))
  (bind (_bblockinghit _binitialoverlap _time _distance _location _impactpoint _normal _impactnormal _physmat _hitactor _hitcomponent _hitbonename) (`GameplayStatics.BreakHitResult` ImpactResult))
  (bind _returnvalue (`Pawn.GetController` (`self.Instigator`)))
  (`PrimitiveComponent.SetCollisionProfileName` (`self.SphereCollision`) "OverlapAll")
  (`|ExecutionSequence`
    (:`then_0`
      (`/Engine/EditorBlueprintResources/StandardMacros.IsValid` _hitcomponent
        (:`Is Valid`
          (if (`SceneComponent.IsSimulatingPhysics` _hitcomponent "None")
            (`PrimitiveComponent.AddImpulseAtLocation` _hitcomponent (0.0 0.0 0.0) _impactpoint "None")))
        (:`Is Not Valid`
          _))
      ;[1 1 1] Spawn FX
      (`|SpawnActorFromClass` "/Game/BP/Effect/BP_ImpactEffect.BP_ImpactEffect_C" (`self.GetTransform` self) "Undefined" "OverrideRootScale" null ImpactResult "NewEnumerator1" (`KismetMathLibrary.VSize` (`self.GetVelocity`)) true 5.0 (`SceneComponent.K2_GetComponentToWorld` (`self.SphereCollision`)) 0.7 null)
      ;[1 1 1] 隐藏 再 销毁
      (`self.SetActorHiddenInGame` self true)
      (`KismetSystemLibrary.Delay` 1.5)
      (`self.K2_DestroyActor`) ; Then destroy this projectile
    )
    (:`then_1`
      (bind _asbp_base_aicharacter (cast `/Game/BP/AI/Monster/BP_BaseAICharacter` _hitactor))
      (`KismetSystemLibrary.PrintString` (`KismetStringLibrary.Conv_NameToString` _hitbonename))
      (if (== _hitbonename "Head")
        (`GameplayStatics.ApplyDamage` _asbp_base_aicharacter (* 2 (`self.Base Damage`)) _returnvalue self)
        (else
          (`GameplayStatics.ApplyDamage` _asbp_base_aicharacter (`self.Base Damage`) _returnvalue self))))))

(fn `UserConstructionScript`
  (`parent.UserConstructionScript`))