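; Game mode that registers joining players, spawns their characters and spawns usable items by type.
; PostLogin records each BPC_PlayerController, gives its player state a numbered name, then possesses a new BP_LittleGirl spawned at the next indexed PlayerStart.
; Every Tick rebuilds the game state's PlayerMsg list from each player's name, score and HP.
; CreateUsable maps types to gun pickup classes; Razer and Not An Item return no class.
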(event `Create Usable`
  (params (Type :type "/Game/BP/Weapon/E_EquipmentType Enum" :default "NewEnumerator0") (Location :type "Vector Structure") (Count :type Integer))
  (`|SpawnActorFromClass` (`self.Get Usable Type` Type) (`KismetMathLibrary.MakeTransform` Location) "Undefined" "OverrideRootScale" null Count null))

(event `self.K2_PostLogin`
  (params (NewPlayer :type "PlayerController Object Reference"))
  ;[1 1 1] Record player on player login
  (bind _asbpc_player_controller (cast `/Game/BP/BPC_PlayerController` NewPlayer)
    (:`then`
      (`KismetArrayLibrary.Array_AddUnique` (`self.PlayerList`) _asbpc_player_controller)
      (`|ExecutionSequence`
        (:`then_0`
          (bind _asbp_player_state (cast `/Game/BP/BP_PlayerState` (`Controller.PlayerState` NewPlayer)))
          (set `/Game/BP/BP_PlayerState.Name` (`KismetStringLibrary.Concat_StrStr` "player" "" (`KismetStringLibrary.Conv_IntToString` (`self.NewVar_0`))) _asbp_player_state)
          (set `self.NewVar_0` (+ (`self.NewVar_0`) 1)))
        (:`then_1`
          (bind _outactors (`GameplayStatics.GetAllActorsOfClass` "/Script/Engine.PlayerStart"))
          (bind _returnvalue (`|SpawnActorFromClass` "/Game/BP/Character/BP_LittleGirl.BP_LittleGirl_C" (`self.GetTransform` (`|GetArrayItem` _outactors (`self.Player Num`))) "AdjustIfPossibleButDontSpawnIfColliding" "OverrideRootScale" null null))
          (`Controller.Possess` NewPlayer _returnvalue)
          (`/Engine/EditorBlueprintResources/StandardMacros.IncrementInt` (`self.Player Num`)))))
    (:`CastFailed`
      (`KismetSystemLibrary.PrintString` "OnPostLogin: cast to desired PlayerController failed"))))

(event `test`
  (`KismetSystemLibrary.PrintString` "1111111111111111111111111111111"))

(event `self.ReceiveTick`
  (params (DeltaSeconds :type "Float (single-precision)"))
  (`self.Refresh PlayerMsgs In Gamestate`))

(fn `Get Usable Type`
  (params (Type :type "/Game/BP/Weapon/E_EquipmentType Enum" :default "NewEnumerator0"))
  (returns (`Type Class` :type "/Game/BP/Projectile/PickUp/BP_UsableBase Class Reference"))
  (switch `/Game/BP/Weapon/E_EquipmentType` Type
    (:`NewEnumerator0`
      (return "/Game/BP/Projectile/PickUp/BP_UsableDefault.BP_UsableDefault_C"))
    (:`NewEnumerator1`
      (return "/Game/BP/Projectile/PickUp/BP_UsableGrenadeGun.BP_UsableGrenadeGun_C"))
    (:`NewEnumerator3`
      _)
    (:`NewEnumerator2`
      _))
  (return null))

(fn `Refresh PlayerMsgs In Gamestate`
  (locals (TempMsg :type "Array of /Game/BP/S_PlayerMsg Structure"))
  (for _array_element (`self.PlayerList`)
    (bind _asbp_player_state (cast `/Game/BP/BP_PlayerState` (`Controller.PlayerState` _array_element)))
    (`KismetArrayLibrary.Array_Add` (`local.TempMsg`) (make `/Game/BP/S_PlayerMsg` (`/Game/BP/BP_PlayerState.Name` _asbp_player_state) (`/Game/BP/BP_PlayerState.Player Score` _asbp_player_state) (`KismetMathLibrary.Conv_IntToDouble` (`/Game/BP/BP_PlayerState.Current HP` _asbp_player_state)))))
  (bind _asbp_game_state (cast `/Game/BP/BP_GameState` (`GameplayStatics.GetGameState`)))
  (set `/Game/BP/BP_GameState.PlayerMsg` (`local.TempMsg`) _asbp_game_state))

(fn `UserConstructionScript`)