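; Game mode for level 02 that runs a multiplayer room lobby, tracking player controllers and their room entries in parallel arrays.
; Login adds an entry after a short delay, marking the first player host and ready, with a numbered fallback for empty names.
; Login and logout push the refreshed list to every controller.
; It also relays kicks by index and broadcasts a wait panel to all players.
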(event `self.ReceiveTick`
  (params (DeltaSeconds :type "Float (single-precision)")))

(event `self.K2_OnLogout`
  (params (ExitingController :type "Controller Object Reference"))
  (for (_array_element _array_index) (`self.Player Controllers`)
    (if (== _array_element ExitingController)
      (break)))
  (`KismetArrayLibrary.Array_Remove` (`self.Player Controllers`) _array_index)
  (`KismetArrayLibrary.Array_Remove` (`self.Player Msgs`) _array_index)
  (`self.Refresh Player List`))

(event `self.K2_PostLogin`
  (params (NewPlayer :type "PlayerController Object Reference"))
  (bind _asbpc_level_02 (cast `/Game/BP/02Level/BPC_level02` NewPlayer))
  (bind _returnvalue (`KismetArrayLibrary.Array_Add` (`self.Player Controllers`) _asbpc_level_02))
  (`KismetSystemLibrary.Delay` 0.2)
  (bind _player_name (`/Game/BP/02Level/BPC_level02.Player Name` _asbpc_level_02))
  (bind _returnvalue_2 (== _returnvalue 0))
  (`KismetArrayLibrary.Array_Add` (`self.Player Msgs`) (make `/Game/BP/02Level/S_PlayerRoomMsgMsg` (select `bool` (`KismetTextLibrary.TextIsEmpty` _player_name) :`false` _player_name :`true` (`KismetTextLibrary.Conv_StringToText` (`KismetStringLibrary.Concat_StrStr` (`KismetTextLibrary.Conv_TextToString` "Player") (`KismetStringLibrary.Conv_IntToString` _returnvalue)))) _returnvalue_2 _returnvalue_2))
  (`self.Refresh Player List`))

(event `Refresh Player List`
  (for (_array_element _array_index) (`self.Player Controllers`)
    (`/Game/BP/02Level/BPC_level02.Setup Player List` _array_element (`self.Player Msgs`) _array_index)))

(event `Kick`
  (params (Index :type Integer))
  (`/Game/BP/02Level/BPC_level02.Kick` (`|GetArrayItem` (`self.Player Controllers`) Index)))

(event `Every One Add Wait Panel`
  (params (Text :type Text))
  (for _array_element (`self.Player Controllers`)
    (`/Game/BP/02Level/BPC_level02.Clinet Show Wait Panel` _array_element Text)))

(fn `UserConstructionScript`)