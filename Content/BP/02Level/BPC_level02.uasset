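; Player controller for the level 02 room lobby, linking each player to the room UI and game mode.
; On BeginPlay it passes the GameInstance player name to a server-named event that stores it.
; Ready changes update BP_GM02's player records, then refresh the list after a short delay.
; It also creates or refreshes WBP_Room, shows wait panels, and handles kicks by opening the start map and destroying the session.
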(event `self.ReceiveBeginPlay`
  (`self.Set Player Name From Client`))

(event `Server Set Player Name`
  (params (NewParam :type Text))
  (set `self.Player Name` NewParam))

(event `Set Player Name From Client`
  (bind _asbp_game_instance (cast `/Game/BP/03Level/BP_GameInstance` (`GameplayStatics.GetGameInstance`)))
  (`self.Server Set Player Name` (`/Game/BP/03Level/BP_GameInstance.Player Name` _asbp_game_instance)))

(event `Kick`
  (`GameplayStatics.OpenLevel` "01StartMap")
  (`DestroySessionCallbackProxy.DestroySession` self))

(event `CustomEvent`
  (params (ServerName :type "Array of /Game/BP/02Level/S_PlayerRoomMsgMsg Structure"))
  (set `self.bShowMouseCursor` true)
  (`/Engine/EditorBlueprintResources/StandardMacros.IsValid` (`self.UI Room Ref`)
    (:`Is Valid`
      _)
    (:`Is Not Valid`
      (bind _returnvalue (`|CreateWidget` "/Game/BP/UI/Room/WBP_Room.WBP_Room_C" null ServerName))
      (bind _output_get (set `self.UI Room Ref` _returnvalue))
      (`UserWidget.AddToViewport` _output_get 0)))
  (`/Game/BP/UI/Room/WBP_Room.Refresh PlayerList` (`self.UI Room Ref`) ServerName))

(event `Setup Player List`
  (params (ServerName :type "Array of /Game/BP/02Level/S_PlayerRoomMsgMsg Structure") (`Player Controller Index` :type Integer))
  (set `self.bShowMouseCursor` true)
  (`/Engine/EditorBlueprintResources/StandardMacros.IsValid` (`self.UI Room Ref`)
    (:`Is Valid`
      _)
    (:`Is Not Valid`
      (bind _returnvalue (`|CreateWidget` "/Game/BP/UI/Room/WBP_Room.WBP_Room_C" null ServerName `Player Controller Index`))
      (bind _output_get (set `self.UI Room Ref` _returnvalue))
      (`UserWidget.AddToViewport` _output_get 0)))
  (`/Game/BP/UI/Room/WBP_Room.Refresh PlayerList` (`self.UI Room Ref`) ServerName))

(event `Server Call GM Refresh Player List`
  (bind _asbp_gm02 (cast `/Game/BP/02Level/BP_GM02` (`GameplayStatics.GetGameMode`)))
  (`/Game/BP/02Level/BP_GM02.Refresh Player List` _asbp_gm02))

(event `Server Set Ready`
  (params (`Player Controller Index` :type Integer) (Ready :type Boolean))
  (bind _asbp_gm02 (cast `/Game/BP/02Level/BP_GM02` (`GameplayStatics.GetGameMode`)))
  (setmembers `/Game/BP/02Level/S_PlayerRoomMsgMsg` :`StructRef` (`|GetArrayItem` (`/Game/BP/02Level/BP_GM02.Player Msgs` _asbp_gm02) `Player Controller Index`) :`Ready` Ready)
  (`KismetSystemLibrary.Delay` 0.2)
  (`/Game/BP/02Level/BP_GM02.Refresh Player List` _asbp_gm02))

(event `Clinet Show Wait Panel`
  (params (Text :type Text))
  (bind _asbp_game_instance (cast `/Game/BP/03Level/BP_GameInstance` (`GameplayStatics.GetGameInstance`)))
  (`/Game/BP/03Level/BP_GameInstance.Show Wait Panel` _asbp_game_instance Text))

(fn `UserConstructionScript`)