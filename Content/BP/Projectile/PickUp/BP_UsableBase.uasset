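; Base pickup actor for usable items that a player collects into the equipment storage of their Weapon.
; PickUp registers the item Type if missing and adds Count, keeping any returned remainder on the actor or destroying it otherwise.
; The same pickup sound plays whether or not the Type can be added.
; SetFocus toggles the mesh's custom depth for highlighting, while older sphere-overlap auto-pickup logic sits disconnected.
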(event `self.ReceiveTick`
  (params (DeltaSeconds :type "Float (single-precision)")))

(event `self.Sphere Collision.OnComponentBeginOverlap`
  (params (OverlappedComponent :type "PrimitiveComponent Object Reference") (OtherActor :type "Actor Object Reference") (OtherComp :type "PrimitiveComponent Object Reference") (OtherBodyIndex :type Integer) (bFromSweep :type Boolean) (SweepResult :type "HitResult Structure (by ref)")))

(event `Pick Up`
  (params (Player :type "/Game/BP/Character/BP_LittleGirl Object Reference"))
  (bind _weapon (`/Game/BP/Character/BP_LittleGirl.Weapon` Player))
  (if (`/Game/BP/Weapon/BP_Weapon.Can Add Type in Current Equipment Msg` _weapon (`self.Type`))
    (if (not (`/Game/BP/Weapon/BP_Weapon.Having A Type in Current Equipment Msg` _weapon (`self.Type`)))
      (`/Game/BP/Weapon/BP_Weapon.Add Type in Current Equipment Msg` _weapon (`self.Type`)))
    (bind _left (`/Game/BP/Weapon/BP_Weapon.Add Current Storage` _weapon (`self.Type`) (`self.Count`)))
    (`GameplayStatics.SpawnSoundAtLocation` (`self.Can Pick Up Sound`) (`self.K2_GetActorLocation`) (struct) 1.0 1.0 0.0 null null)
    (if (> _left 0)
      (set `self.Count` _left)
      (else
        (`self.K2_DestroyActor`)))
    (else
      (`GameplayStatics.SpawnSoundAtLocation` (`self.Can Pick Up Sound`) (`self.K2_GetActorLocation`) (struct) 1.0 1.0 0.0 null null))))

(fn `Set Focus`
  (params (Focus :type Boolean))
  (`PrimitiveComponent.SetRenderCustomDepth` (`self.StaticMesh`) Focus))

(fn `UserConstructionScript`)