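; BP_GunGrenade is a grenade projectile that explodes on its first bounce, then destroys itself.
; The bounce switches its collision to overlap and passes hit data through a DoOnce to Boom.
; Boom plays particles, sound and camera shake, applies radial damage and impulse, and draws a debug sphere.
; It also fakes craters by scattering randomly scaled, short-lived BP_DefaultProjectile actors flagged as IsHelpGrenade.
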(event `Boom`
  (bind _impact_point (`self.Impact Point`))
  (`GameplayStatics.SpawnEmitterAtLocation` "/Game/Asset/BallisticsVFX/Particles/Explosive/Explosion_GrenadeLauncher_1.Explosion_GrenadeLauncher_1" (`self.Location`) (`KismetMathLibrary.MakeRotFromZ` (* (`KismetMathLibrary.RandomUnitVectorInConeInRadians` (`KismetMathLibrary.GetDirectionUnitVector` (`self.Impact Normal`)) (`self.Explosion Angle Variance VFX`)) -1.0)) (0.2 0.2 0.2))
  (`GameplayStatics.PlayWorldCameraShake` "/Game/BP/Projectile/ExplosionShake.ExplosionShake_C" (`self.Location`) 0.0 5000.0)
  (`GameplayStatics.SpawnSoundAtLocation` "/Game/Asset/BallisticsVFX/SFX/Explodes/Explosions.Explosions" (`self.Location`) (struct) 0.75 1.0 0.0 "/Game/Asset/BallisticsVFX/SFX/Attentuations/Gun_Attenuation.Gun_Attenuation" null)
  (`KismetSystemLibrary.DrawDebugSphere` _impact_point 400.0 12 (struct :`R` 1.0 :`A` 1.0) 10.0)
  (`GameplayStatics.ApplyRadialDamage` :`BaseDamage` (`self.Base Damage`) :`Origin` _impact_point :`DamageRadius` 400.0 :`DamageCauser` self :`InstigatedByController` (`Pawn.GetController` (`self.Instigator`)) :`DamagePreventionChannel` "ECC_Camera")
  (`PrimitiveComponent.AddRadialImpulse` (`self.Hit Comp`) _impact_point 500.0 1000000.0 "RIF_Linear" false)
  ;[1 1 1] 生成子弹 伪装弹坑
  (for _ (range 21)
    (bind _returnvalue (`|SpawnActorFromClass` "/Game/BP/Projectile/Projectile/BP_DefaultProjectile.BP_DefaultProjectile_C" (`KismetMathLibrary.MakeTransform` (`self.Location`) (`KismetMathLibrary.Conv_VectorToRotator` (`KismetMathLibrary.RandomUnitVectorInEllipticalConeInDegrees` (`self.Impact Normal`) 179.0 179.0)) (`KismetMathLibrary.MakeVector` (`KismetMathLibrary.RandomFloatInRange` 0.0 2.0) (`KismetMathLibrary.RandomFloatInRange` 0.0 2.0) (`KismetMathLibrary.RandomFloatInRange` 0.0 2.0))) "AdjustIfPossibleButAlwaysSpawn" "OverrideRootScale" null true (`KismetMathLibrary.RandomFloatInRange` 50.0 100.0) 20.0 null)) ; Spawn projectile
    (`self.SetLifeSpan` _returnvalue (`KismetMathLibrary.RandomFloatInRange` 0.0 1.5)))
  (`self.K2_DestroyActor`))

(event `self.ProjectileMovement.OnProjectileBounce`
  (params (ImpactResult :type "HitResult Structure (by ref)") (ImpactVelocity :type "Vector Structure (by ref)"))
  (bind (_bblockinghit _binitialoverlap _time _distance _location _impactpoint _normal _impactnormal _physmat _hitactor _hitcomponent) (`GameplayStatics.BreakHitResult` ImpactResult))
  (`PrimitiveComponent.SetCollisionProfileName` (`self.SphereCollision`) "OverlapAll")
  (`/Engine/EditorBlueprintResources/StandardMacros.DoOnce` false
    (:`Completed`
      (set `self.Location` _location)
      (set `self.Impact Point` _impactpoint)
      (set `self.Impact Normal` _impactnormal)
      (set `self.Hit Comp` _hitcomponent)
      (`self.Boom`))))

(fn `UserConstructionScript`
  (`parent.UserConstructionScript`))