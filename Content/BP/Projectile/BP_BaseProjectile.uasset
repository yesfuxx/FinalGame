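; BP_BaseProjectile is a projectile Blueprint, named as a base, that sets up launch speed and damage when constructed.
; On the server only, its construction script copies InitialSpeed into the ProjectileMovement component and randomizes BaseDamage by a proportional ± DamageOffset, rounded to a whole number.
; The event graph has no active logic, so overlap, hit and damage application are not handled in these graphs.
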(event `self.ReceiveBeginPlay`)

(fn `Set Speed`
  (set `ProjectileMovementComponent.InitialSpeed` (`self.Initial Speed`) (`self.ProjectileMovement`)))

(fn `UserConstructionScript`
  (bind _damage_offset (`self.Damage Offset`))
  (if (`KismetSystemLibrary.IsServer`)
    (`self.Set Speed`)
    (set `self.Base Damage` (`KismetMathLibrary.Conv_IntToDouble` (`KismetMathLibrary.Round` (+ (* (`self.Base Damage`) (`KismetMathLibrary.RandomFloatInRange` (* _damage_offset -1.0) _damage_offset)) (`self.Base Damage`)))))))