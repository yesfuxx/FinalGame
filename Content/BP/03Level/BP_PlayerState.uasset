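; Player state that holds each player's name, score, HP and death flag, with functions to add score and heal or damage within HP limits.
; On BeginPlay it caches the game mode and sends the name saved in the game instance through a server-named event.
; RepNotifies on name, score and HP call the game mode to refresh player list parameters.
; The client low-HP check casts to BP_LittleGirl, but its breathing sound call is disconnected.
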(event `self.ReceiveBeginPlay`
  (`|ExecutionSequence`
    (:`then_0`
      (bind _asbp_game_mode (cast `/Game/BP/03Level/BP_GameMode` (`GameplayStatics.GetGameMode`)))
      (set `self.Gamemode` _asbp_game_mode))
    (:`then_1`
      (`self.Set Player Name`))))

(event `Set Player Name`
  (bind _asbp_game_instance (cast `/Game/BP/03Level/BP_GameInstance` (`GameplayStatics.GetGameInstance`)))
  (`self.Server Set Player Name` (`/Game/BP/03Level/BP_GameInstance.Player Name` _asbp_game_instance)))

(event `Server Set Player Name`
  (params (InText :type "Text (by ref)"))
  (set `self.Name` (`KismetTextLibrary.Conv_TextToString` InText)))

(event `Update Player List Msg`
  (`/Game/BP/03Level/BP_GameMode.Update Player List Params` (`self.Gamemode`)))

(fn `Add HP`
  (params (`Add HP Value` :type Integer))
  (bind _max_hp (`self.Max HP`))
  (bind _returnvalue (+ `Add HP Value` (`self.Current HP`)))
  (if (> _returnvalue _max_hp)
    (set `self.Current HP` _max_hp)
    (else
      (set `self.Current HP` _returnvalue))))

(fn `Add Score`
  (params (`A Score` :type Integer))
  (set `self.Player Score` (+ `A Score` (`self.Player Score`))))

(fn `Cut HP`
  (params (`Cut HP Value` :type Integer))
  (bind _returnvalue (- (`self.Current HP`) `Cut HP Value`))
  (if (<= _returnvalue 0)
    (set `self.Current HP` 0)
    (set `self.Death` true)
    (else
      (set `self.Current HP` _returnvalue))))

(fn `OnRep_Current HP`
  (bind _current_hp (`self.Current HP`))
  (`|ExecutionSequence`
    (:`then_0`
      (`self.Update Player List Msg`))
    (:`then_1`
      (if (`KismetSystemLibrary.IsServer`)
        _
        (elif (<= _current_hp 20)
          (if (`KismetMathLibrary.InRange_IntInt` _current_hp 0 20 false)
            (bind _asbp_little_girl (cast `/Game/BP/Character/BP_LittleGirl` (`GameplayStatics.GetPlayerPawn` 0)))))))))

(fn `OnRep_Name`
  (`self.Update Player List Msg`))

(fn `OnRep_Player Score`
  (`self.Update Player List Msg`))

(fn `UserConstructionScript`)