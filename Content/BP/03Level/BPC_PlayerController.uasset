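; BPC_PlayerController is the level's player controller, acting as the bridge to each player's UI for the player list, level number and game-over screen.
; It forwards player-list updates to the main widget, revealing the list when the GameState reports more than one player.
; Game over is shown through BP_GameInstance, then the cursor appears and the controlled BP_LittleGirl's HUD is hidden.
; A UI-only input mode call is left unconnected.
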(event `self.ReceiveBeginPlay`
  (bind _asbp_game_state (cast `/Game/BP/03Level/BP_GameState` (`GameplayStatics.GetGameState`)))
  (set `self.GameState Ref` _asbp_game_state))

(event `Refresh Player List`
  (params (NewParam :type Integer))
  (bind _wbp_main (`self.WBP_Main`))
  (bind _wbp_playmsglist (`/Game/BP/UI/Game/WBP_Main.WBP_PlayMsgList` _wbp_main))
  (`/Engine/EditorBlueprintResources/StandardMacros.IsValid` _wbp_main
    (:`Is Valid`
      (`/Game/BP/UI/Game/PlayList/WBP_PlayMsgList.Refresh Items` _wbp_playmsglist NewParam)
      (if (> (`/Game/BP/03Level/BP_GameState.Player Num` (`self.GameState Ref`)) 1)
        (`Widget.SetVisibility` _wbp_playmsglist "Visible")))))

(event `Refresh Player List Params`
  (params (msgs :type "Array of /Game/BP/03Level/S_PlayerMsg Structure"))
  (bind _wbp_main (`self.WBP_Main`))
  (bind _wbp_playmsglist (`/Game/BP/UI/Game/WBP_Main.WBP_PlayMsgList` _wbp_main))
  (`/Engine/EditorBlueprintResources/StandardMacros.IsValid` _wbp_main
    (:`Is Valid`
      (`/Engine/EditorBlueprintResources/StandardMacros.IsValid` _wbp_playmsglist
        (:`Is Valid`
          (`/Game/BP/UI/Game/PlayList/WBP_PlayMsgList.Refresh Player List Params` _wbp_playmsglist msgs))))))

(event `Show UI GameOver`
  (params (msgs :type "Array of /Game/BP/UI/Game/GameOver/S_OverMsgMsg Structure"))
  (bind _asbp_game_instance (cast `/Game/BP/03Level/BP_GameInstance` (`GameplayStatics.GetGameInstance`)))
  (`/Game/BP/03Level/BP_GameInstance.Show UI GameOver` _asbp_game_instance msgs)
  (set `self.bShowMouseCursor` true)
  (bind _asbp_little_girl (cast `/Game/BP/Character/BP_LittleGirl` (`self.K2_GetPawn` self)))
  (`Widget.SetVisibility` (`/Game/BP/Character/BP_LittleGirl.Main UI` _asbp_little_girl) "Hidden"))

(event `Client UI LevelNum Show`
  (`/Game/BP/UI/Game/WBP_LevelNum.Play Fade` (`/Game/BP/UI/Game/WBP_Main.WBP_LevelNum` (`self.WBP_Main`))))

(fn `UserConstructionScript`)